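; Prototype game mode for a five-round duel in which player and AI each use a sequence of moves numbered 1 to 3.
; BeginPlay rolls the AI's moves, then Tick waits for PcontrollerXD to be ready and runs NacoCheck once.
; NacoCheck classifies each pair through the Cthulu macro, which gives 2v1 the same case as 1v3.
; Every handled case prints its label and costs the player one life, with no win logic.
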(event `self.ReceiveBeginPlay`
  (bind _aifightingarray (`self.AIFightingArray`))
  (set `self.VidaAI` 4)
  (set `self.VidaPlayer` 4)
  (set `self.StartedChecking` true)
  (for _ (range 5)
    (`KismetArrayLibrary.Array_Add` _aifightingarray (`KismetMathLibrary.RandomIntegerInRange` 1 3)))
  (for _array_element _aifightingarray
    (`KismetSystemLibrary.PrintString` (`KismetStringLibrary.Conv_IntToString` _array_element))))

(event `NacoCheck`
  (bind _aspcontroller_xd (cast `/Game/Blueprints/PcontrollerXD` (`GameplayStatics.GetPlayerController` 0)))
  (for _index (range 5)
    (bind _output_get (set `self.PlayerFightingInst` (`|GetArrayItem` (`/Game/Blueprints/PcontrollerXD.FightingArray` _aspcontroller_xd) _index)))
    (bind _output_get_2 (set `self.AIfightingInst` (`|GetArrayItem` (`self.AIFightingArray`) _index)))
    (`self.Cthulu` _output_get _output_get_2 _output_get _output_get_2 _output_get _output_get_2
      (:`then`
        _)
      (:`then2`
        _)
      (:`then3`
        _)
      (:`then4`
        _)
      (:`then5`
        _)
      (:`then6`
        _)
      (:`then7`
        _)
      (:`then8`
        _)
      (:`then9`
        _))
    (switch `int` (`self.FightCase`)
      (:`0`
        (`KismetSystemLibrary.PrintString` "1v1"))
      (:`1`
        (`KismetSystemLibrary.PrintString` "1v2"))
      (:`2`
        (`KismetSystemLibrary.PrintString` "1v3"))
      (:`3`
        (`KismetSystemLibrary.PrintString` "2v1"))
      (:`4`
        (`KismetSystemLibrary.PrintString` "2v2"))
      (:`5`
        (`KismetSystemLibrary.PrintString` "2v3"))
      (:`6`
        (`KismetSystemLibrary.PrintString` "3v1"))
      (:`7`
        (`KismetSystemLibrary.PrintString` "3v2"))
      (:`8`
        (`KismetSystemLibrary.PrintString` "3v3")))
    (`self.PierdeVidaPlayer`)))

(event `self.ReceiveTick`
  (params (DeltaSeconds :type "Float (single-precision)"))
  (bind _aspcontroller_xd (cast `/Game/Blueprints/PcontrollerXD` (`GameplayStatics.GetPlayerController` 0)))
  (if (and (`/Game/Blueprints/PcontrollerXD.IsReady2Fight` _aspcontroller_xd) (`self.StartedChecking`))
    (set `self.StartedChecking` false)
    (`self.NacoCheck`)))

(fn `PierdeVidaPlayer`
  (bind _aspcontroller_xd (cast `/Game/Blueprints/PcontrollerXD` (`GameplayStatics.GetPlayerController` 0)))
  (set `/Game/Blueprints/PcontrollerXD.VidaPlayer` (- (`/Game/Blueprints/PcontrollerXD.VidaPlayer` _aspcontroller_xd) 1.0) _aspcontroller_xd))

(fn `UserConstructionScript`)