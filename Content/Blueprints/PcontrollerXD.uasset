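; Player controller that records a sequence of five player decisions, apparently in preparation for a fight.
; BeginPlay initializes player life, shows the Robot_Lifes widget and clears the ready flag.
; Three Decision inputs each append their number to FightingArray.
; Tick watches for exactly five entries, then prints them once and sets IsReady2Fight; no fight resolution or array reset happens here.
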(event `self.ReceiveTick`
  (params (DeltaSeconds :type "Float (single-precision)"))
  (if (== (`KismetArrayLibrary.Array_Length` (`self.FightingArray`)) 5)
    (if (not (`self.IsReady2Fight`))
      (for _array_element (`self.FightingArray`)
        (`KismetSystemLibrary.PrintString` (`KismetStringLibrary.Conv_IntToString` _array_element)))
      (set `self.IsReady2Fight` true))))

(event `self.ReceiveBeginPlay`
  (set `self.VidaPlayer` 6.0)
  (bind _returnvalue (`|CreateWidget` "/Game/Boch/Robot_Lifes.Robot_Lifes_C"))
  (`UserWidget.AddToPlayerScreen` _returnvalue 0)
  (set `self.IsReady2Fight` false))

(event `InputAction|Decision1`
  (params (Key :type "Key Structure"))
  ;[1 1 1] Inputs
  (:`Pressed`
    (`KismetArrayLibrary.Array_Add` (`self.FightingArray`) 1)))

(event `InputAction|Decision2`
  (params (Key :type "Key Structure"))
  ;[1 1 1] Inputs
  (:`Pressed`
    (`KismetArrayLibrary.Array_Add` (`self.FightingArray`) 2)))

(event `InputAction|Decision3`
  (params (Key :type "Key Structure"))
  ;[1 1 1] Inputs
  (:`Pressed`
    (`KismetArrayLibrary.Array_Add` (`self.FightingArray`) 3)))

(fn `UserConstructionScript`)